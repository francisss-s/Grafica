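; Enemy actor that drains Power from a BP-class actor through a damage zone and flags detection through a vision zone.
; Tick and ZonaDaño overlap share a half-second Delay, then cast the overlapped actor and, unless BpRef is dead, set its Power to BpRef's minus a fixed amount and pass that to PowerDamage.
; A ZonaVision hit by a BP actor sets Detect, which is not read here.
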(event `self.ReceiveBeginPlay`)

(event `self.ReceiveTick`
  (params (DeltaSeconds :type "Float (single-precision)"))
  (bind _bpref (`self.BpRef`))
  (`KismetSystemLibrary.Delay` 0.5 :!label _label)
  (bind _asbp (cast `/Game/Blueprints/BP` (stale `self.ZonaDaño.OnComponentBeginOverlap` OtherActor)))
  (if (not (`/Game/Blueprints/BP.Is Dead` _bpref))
    (bind _output_get (set `/Game/Blueprints/BP.Power` (- (`/Game/Blueprints/BP.Power` _bpref) 10.0) _asbp))
    (`/Game/Blueprints/BP.Power Damage` _asbp _output_get)))

(event `self.ZonaDaño.OnComponentBeginOverlap`
  (params (OverlappedComponent :type "PrimitiveComponent Object Reference") (OtherActor :type "Actor Object Reference") (OtherComp :type "PrimitiveComponent Object Reference") (OtherBodyIndex :type Integer) (bFromSweep :type Boolean) (SweepResult :type "HitResult Structure (by ref)"))
  (goto _label))

(event `self.ZonaVision.OnComponentHit`
  (params (HitComponent :type "PrimitiveComponent Object Reference") (OtherActor :type "Actor Object Reference") (OtherComp :type "PrimitiveComponent Object Reference") (NormalImpulse :type "Vector Structure") (Hit :type "HitResult Structure (by ref)"))
  (cast `/Game/Blueprints/BP` OtherActor)
  (set `self.Detect` true))

(fn `UserConstructionScript`)