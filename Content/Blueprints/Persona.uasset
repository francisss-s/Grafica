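; Player character (Persona) with side-to-side movement and a two-camera toggle.
; MovementUpdate maps the MoveRigth axis to world X in PuzzleMode, otherwise to the actor's forward vector; the axis event itself passes a zero direction.
; C compares the camera manager's location to Camera1, then blends the view to the CamaraHijo child actor or back to itself.
; EnableDisableInput always enables input, ignoring its Enable parameter.
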(event `self.ReceiveBeginPlay`)

(event `Enable Disable Input`
  (params (Enable :type Boolean))
  (bind _returnvalue (`GameplayStatics.GetPlayerController` 0))
  ;[1 1 1] Enable Disable Input
  (if true
    (`self.EnableInput` _returnvalue)
    (else
      (`self.DisableInput` _returnvalue))))

(event `InputAxis|MoveRigth`
  (params (AxisValue :type "Float (single-precision)"))
  (`self.AddMovementInput` (0.0 0.0 0.0) AxisValue))

(event `Movement Update`
  ;[1 1 1] Movement Update
  (if (`self.Puzzle Mode`)
    (set `self.Move Direction` (`KismetMathLibrary.MakeVector` (`self.GetInputAxisValue`)))
    (else
      (set `self.Move Direction` (`KismetMathLibrary.Normal` (* (`self.GetActorForwardVector`) (`self.GetInputAxisValue`))))))
  (`self.AddMovementInput` (`KismetMathLibrary.Normal` (`self.Move Direction`))))

(event `Key|C`
  (params (Key :type "Key Structure"))
  ;[1 1 1] Cambio de camara
  (:`Pressed`
    (if (== (`SceneComponent.K2_GetComponentLocation` (`PlayerCameraManager.TransformComponent` (`GameplayStatics.GetPlayerCameraManager` 0))) (`SceneComponent.K2_GetComponentLocation` (`self.Camera1`)))
      (`self.Camara 1`)
      (else
        (`self.Camara 2`)))))

(fn `Camara 1`
  (`PlayerController.SetViewTargetWithBlend` (`GameplayStatics.GetPlayerController` 0) (`ChildActorComponent.ChildActor` (`self.CamaraHijo`)) 0.5 "VTBlend_Linear" 0.0 false))

(fn `Camara 2`
  (`PlayerController.SetViewTargetWithBlend` (`GameplayStatics.GetPlayerController` 0) self 0.5 "VTBlend_Linear" 0.0 false))

(fn `UserConstructionScript`)