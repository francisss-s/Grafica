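; Player character Blueprint with axis-driven movement, wall jumping, a timed attack, and energy and power stats.
; Tick applies movement along world X in PuzzleMode or the actor's forward axis otherwise, and regenerates energy.
; Airborne jumps line-trace for walls and launch away; PowerDamage flags death and switches off the ball material at zero power.
; The C key blends the view between the character and a child-actor camera.
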(event `self.ReceiveBeginPlay`)

(event `self.ReceiveTick`
  (params (DeltaSeconds :type "Float (single-precision)"))
  (`self.Movement Update`)
  (`self.Movement Update`)
  (`self.Energy Damage` -25.0))

(event `Enable Disable Input`
  (params (Enable :type Boolean))
  (bind _returnvalue (`GameplayStatics.GetPlayerController` 0))
  ;[1 1 1] Enable Disable Input
  (if true
    (`self.EnableInput` _returnvalue)
    (else
      (`self.DisableInput` _returnvalue))))

(event `Movement Update`
  ;[1 1 1] Movement Update
  (if (`self.Puzzle Mode`)
    (set `self.Move Direction` (`KismetMathLibrary.MakeVector` (`self.GetInputAxisValue`)))
    (else
      (set `self.Move Direction` (`KismetMathLibrary.Normal` (* (`self.GetActorForwardVector`) (`self.GetInputAxisValue`))))))
  (`self.AddMovementInput` (`KismetMathLibrary.Normal` (`self.Move Direction`))))

(event `InputAction|Jump`
  (params (Key :type "Key Structure"))
  (bind _returnvalue (`self.GetActorForwardVector`))
  (bind _returnvalue_x (`KismetMathLibrary.BreakVector` (`self.K2_GetActorLocation`)))
  ;[1 1 1] Player Jump
  (:`Pressed`
    (if (`NavMovementComponent.IsFalling` (`self.CharacterMovement`))
      (bind (_outhit _returnvalue_2) (`KismetSystemLibrary.LineTraceSingle` (- (`self.K2_GetActorLocation`) (* _returnvalue (+ (`CapsuleComponent.GetScaledCapsuleRadius` (`self.CapsuleComponent`)) 10.0))) (+ (`self.K2_GetActorLocation`) (* _returnvalue (+ (`CapsuleComponent.GetScaledCapsuleRadius` (`self.CapsuleComponent`)) 10.0))) "TraceTypeQuery1"))
      (if _returnvalue_2
        (`SkeletalMeshComponent.PlayAnimation` (`self.Mesh`) "/Game/Personaje/Deslizar_Anim.Deslizar_Anim" false)
        (`self.LaunchCharacter` (`KismetMathLibrary.MakeVector` (* (`KismetMathLibrary.SignOfFloat` (- _returnvalue_x (.x (`.Location` (`GameplayStatics.BreakHitResult` _outhit))))) 2500.0) 0.0 3000.0))
        (`KismetSystemLibrary.Delay` 0.5)
        (`SkeletalMeshComponent.SetAnimationMode` (`self.Mesh`) "AnimationBlueprint"))
      (else
        (`self.Jump`)))))

(event `Power Damage`
  (params (Power :type "Float (double-precision)"))
  ;[1 1 1] Power Damage
  (set `self.Power` (`KismetMathLibrary.FClamp` (- (`self.Power`) (* Power (`GameplayStatics.GetWorldDeltaSeconds`))) 0.0 100.0))
  (if (<= (`self.Power`) 0.0)
    (set `self.Is Dead` true)
    (`self.Change Ball Material Color` "IsOn")
    (`self.Enable Disable Input` false)))

(event `Energy Damage`
  (params (Damage :type "Float (double-precision)"))
  ;[1 1 1] Energy damage (positivo = daño, negativo = curacion)
  (set `self.Energy` (`KismetMathLibrary.FClamp` (- (`self.Energy`) (* Damage (`GameplayStatics.GetWorldDeltaSeconds`))) 0.0 100.0)))

(event `Key|C`
  (params (Key :type "Key Structure"))
  ;[1 1 1] Cambio de camara
  (:`Pressed`
    (if (== (`SceneComponent.K2_GetComponentLocation` (`PlayerCameraManager.TransformComponent` (`GameplayStatics.GetPlayerCameraManager` 0))) (`SceneComponent.K2_GetComponentLocation` (`self.Camera`)))
      (`self.Camara 1`)
      (else
        (`self.Camara 2`)))))

(event `InputAction|Atack`
  (params (Key :type "Key Structure"))
  ;[1 1 1] Atack
  (:`Pressed`
    (set `self.Atk` true)
    (`KismetSystemLibrary.Delay` 1.0)
    (set `self.Atk` false))
  (:`Released`
    (`SkeletalMeshComponent.PlayAnimation` (`self.Mesh`) "/Game/Personaje/Wate_Anim.Wate_Anim" false)
    (`KismetSystemLibrary.Delay` 1.0)
    (`SkeletalMeshComponent.SetAnimationMode` (`self.Mesh`) "AnimationBlueprint")))

(fn `Camara 1`
  (`PlayerController.SetViewTargetWithBlend` (`GameplayStatics.GetPlayerController` 0) (`ChildActorComponent.ChildActor` (`self.CamaraHijo`)) 0.5 "VTBlend_Linear" 0.0 false))

(fn `Camara 2`
  (`PlayerController.SetViewTargetWithBlend` (`GameplayStatics.GetPlayerController` 0) self 0.5 "VTBlend_Linear" 0.0 false))

(fn `Change Ball Material Color`
  (params (`Param Name` :type Name) (Value :type "Float (double-precision)")))

(fn `UserConstructionScript`)